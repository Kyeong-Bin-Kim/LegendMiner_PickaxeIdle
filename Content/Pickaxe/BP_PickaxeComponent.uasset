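; BP_PickaxeComponent manages a pickaxe's data and appearance based on its level.
; UpdatePickaxeData looks up the data table row named after PickaxeLevel and stores it, printing a message if none is found.
; SetPickaxeMesh applies the stored mesh and material, then deactivates the Niagara effect and reactivates it with the row's effect asset if valid.
; The event graph is empty, so neither function is called within the component.
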(event EventBeginPlay)

(event EventTick
  (params (DeltaSeconds :type Float%20%28single-precision%29)))

(fn UpdatePickaxeData
  (bind _returnvalue (Utilities|GetDataTableRow (Variables|Default|GetDT_PickaxeData) (Utilities|String|StringToName (Utilities|String|ToString(Integer) (Variables|Default|GetPickaxeLevel))))
    (:then
      (Variables|Default|SetPickaxeData _returnvalue))
    (:RowNotFound
      (Development|PrintString "Pickaxe Data Not Found!"))))

(fn SetPickaxeMesh
  (bind _staticmeshcomponent (Variables|디폴트|GetStaticMeshComponent))
  (bind _pickaxedata (Variables|Default|GetPickaxeData))
  (bind _pickaxeeffectcomponent_ (Variables|Default|GetPickaxeEffectComponent%20))
  (bind _pickaxeeffectcomponent__2 (Variables|Default|GetPickaxeEffectComponent%20))
  (Components|StaticMesh|SetStaticMesh _staticmeshcomponent (.mesh _pickaxedata))
  (Rendering|Material|SetMaterial _staticmeshcomponent 0 (.material _pickaxedata))
  (Utilities|IsValid _pickaxeeffectcomponent_
    (:Is%20Valid
      (Components|Activation|Deactivate _pickaxeeffectcomponent_)
      (Utilities|IsValid (.effect _pickaxedata)
        (:Is%20Valid
          (Utilities|IsValid _pickaxeeffectcomponent__2
            (:Is%20Valid
              (Class|NiagaraComponent|SetAsset _pickaxeeffectcomponent__2 (.effect _pickaxedata) true)
              (Components|Activation|Activate (Variables|Default|GetPickaxeEffectComponent%20) false))))))))